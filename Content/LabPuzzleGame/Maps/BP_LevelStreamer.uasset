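; BP_LevelStreamer is a level marker that reports its level index and spawn point to BP_GameInstance.
; On BeginPlay it registers the location of its Spawn reference, if valid, under CurrentLevelIndex.
; Activate checks and clears an IsActive flag, so it fires once while armed, then sets the game instance's current level index.
; The graph performs no streaming itself, and its IsActive function always returns false.
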(event EventBeginPlay
  (bind _spawn (Variables|Default|GetSpawn))
  (bind _asbp_game_instance (Utilities|Casting|CastToBP_GameInstance (Game|GetGameInstance)))
  (Utilities|IsValid _spawn
    (:Is%20Valid
      (Default|CallOnSaveLevelSpawnLocation _asbp_game_instance (Variables|Default|GetCurrentLevelIndex) (Transformation|GetActorLocation _spawn)))))

(event EventActivate
  (params (Type :type EActivationType%20Enum :default "NewEnumerator0"))
  (if (Variables|Default|GetbIsActive)
    (Variables|Default|SetbIsActive false)
    (bind _asbp_game_instance (Utilities|Casting|CastToBP_GameInstance (Game|GetGameInstance)))
    (Default|CallOnLevelIndexSet _asbp_game_instance (Variables|Default|GetCurrentLevelIndex))))

(fn ConstructionScript)

(fn IsActive
  (return false))