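; BP_AntiexpropriationField is a switchable puzzle field that sends an expropriate-try message to actors entering its box volume while active.
; On BeginPlay it sets the box scale and, if active, starts its Niagara effect and messages any BP_BaseCube already inside.
; Activate routes the requested type through ActivationSwitch: turning on repeats that effect and cube sweep, while turning off clears the flag and stops the effect.
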(event OnComponentBeginOverlap(Box)
  (params (OverlappedComponent :type Primitive%20Component%20Object%20Reference) (OtherActor :type Actor%20Object%20Reference) (OtherComp :type Primitive%20Component%20Object%20Reference) (OtherBodyIndex :type Integer) (bFromSweep :type Boolean) (SweepResult :type Hit%20Result%20Structure%20%28by%20ref%29))
  (if (Variables|Default|GetbIsActive)
    (Class|BPINonExpropriable|ExpropriateTry(Message) OtherActor)))

(event EventBeginPlay
  (Transformation|SetRelativeScale3D (Variables|Default|GetBox) "2.000000,1.000000,1.500000")
  (if (Variables|Default|GetbIsActive)
    (Components|Activation|Activate (Variables|Default|GetNS_AntiexpropriationField) false)
    (for _array_element (Collision|GetOverlappingActors (Variables|Default|GetBox) "/Game/LabPuzzleGame/PuzzleElements/PuzzleCubes/BP_BaseCube.BP_BaseCube_C" :!class /Script/Engine.PrimitiveComponent)
      (Class|BPINonExpropriable|ExpropriateTry(Message) _array_element))))

(event EventActivate
  (params (Type :type EActivationType%20Enum :default "NewEnumerator0"))
  (bind _ns_antiexpropriationfield (Variables|Default|GetNS_AntiexpropriationField))
  (Utilities|ActivationSwitch Type (Variables|Default|GetbIsActive)
    (:TurnOn
      (Variables|Default|SetbIsActive true)
      (Components|Activation|Activate _ns_antiexpropriationfield false)
      (for _array_element (Collision|GetOverlappingActors (Variables|Default|GetBox) "/Game/LabPuzzleGame/PuzzleElements/PuzzleCubes/BP_BaseCube.BP_BaseCube_C" :!class /Script/Engine.PrimitiveComponent)
        (Class|BPINonExpropriable|ExpropriateTry(Message) _array_element)))
    (:TurnOff
      (Variables|Default|SetbIsActive false)
      (Components|Activation|Deactivate _ns_antiexpropriationfield))))

(fn ConstructionScript)

(fn IsActive
  (return false))