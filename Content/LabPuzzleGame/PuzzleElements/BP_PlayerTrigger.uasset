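; BP_PlayerTrigger is a puzzle trigger volume that activates its linked elements when something begins overlapping its Box.
; The overlap event casts to BP_VRPawn, but Trigger runs whatever the result, so firing is not limited to the player.
; Trigger calls ActivateLinked while Active is set; with Once enabled, it then clears Active and prints the StaticMesh world location.
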(event OnComponentBeginOverlap(Box)
  (params (OverlappedComponent :type Primitive%20Component%20Object%20Reference) (OtherActor :type Actor%20Object%20Reference) (OtherComp :type Primitive%20Component%20Object%20Reference) (OtherBodyIndex :type Integer) (bFromSweep :type Boolean) (SweepResult :type Hit%20Result%20Structure%20%28by%20ref%29))
  (Utilities|Casting|CastToBP_VRPawn OtherActor
    (:then
      _)
    (:CastFailed
      _))
  (CallFunction|Trigger))

(fn ConstructionScript)

(fn Trigger
  (if (Variables|Default|GetbActive)
    (CallFunction|ActivateLinked)
    (if (Variables|Default|GetbOnce)
      (Variables|Default|SetbActive false)
      (Development|PrintString (Utilities|String|ToString(Vector) (Transformation|GetWorldLocation (Variables|Default|GetStaticMesh)))))))