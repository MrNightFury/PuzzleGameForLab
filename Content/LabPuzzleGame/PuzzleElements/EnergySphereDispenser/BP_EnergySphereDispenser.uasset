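; Puzzle element that launches a BP_EnergySphere from its ShootLocation along that component's forward vector, with a configurable lifetime.
; It fires on BeginPlay if active or on Activate, which switches an already active reshooting dispenser off instead.
; Each sphere receives a dispenser reference, and Shoot takes a sphere-died flag to support continuous respawning or one-shot firing via ReshootWhenSphereDie.
; Reset deactivates the stored sphere and the dispenser.
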(event EventBeginPlay
  (if (Variables|Default|GetbIsActive)
    (CallFunction|Shoot false)))

(event EventActivate
  (params (Type :type EActivationType%20Enum :default "NewEnumerator0"))
  (if (and (Variables|Default|GetbIsActive) (Variables|Default|GetbReshootWhenSphereDie))
    (Variables|Default|SetbIsActive false)
    (else
      (Variables|Default|SetbIsActive true)
      (CallFunction|Shoot false))))

(fn ConstructionScript)

(fn Shoot
  (params (bIsSphereDied :type Boolean))
  (bind _shootlocation (Variables|Default|GetShootLocation))
  (if (Variables|Default|GetbIsActive)
    (if (and bIsSphereDied (not (Variables|Default|GetbReshootWhenSphereDie)))
      (Variables|Default|SetbIsActive false)
      (else
        (bind _returnvalue (Game|SpawnActorfromClass "/Game/LabPuzzleGame/PuzzleElements/EnergySphere/BP_EnergySphere.BP_EnergySphere_C" (Math|Transform|MakeTransform (Transformation|GetWorldLocation _shootlocation)) "AlwaysSpawn" "MultiplyWithRoot" 0 (* (Math|Vector|GetForwardVector (Transformation|GetWorldRotation _shootlocation)) 1e+02) self (Variables|Default|GetSpheresLifetime) 0))
        (Variables|Default|SetSphere _returnvalue)
        (if (not (Variables|Default|GetbReshootWhenSphereDie))
          (Variables|Default|SetbIsActive false))))))

(fn Reset
  (Default|Deactivate (Variables|Default|GetSphere))
  (Variables|Default|SetbIsActive false))

(fn IsActive
  (return false))