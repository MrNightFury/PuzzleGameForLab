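; BP_SphereDissolver is a puzzle element whose dissolving field destroys energy spheres that touch it.
; While active, its box kills entering BP_EnergySphere actors that have a FieldsCount of zero.
; Activate events pass through optional reversal and a switch that toggles the state and Niagara effect.
; Turning on, or starting active, also kills every sphere already inside, without checking FieldsCount.
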(event OnComponentBeginOverlap(Box)
  (params (OverlappedComponent :type Primitive%20Component%20Object%20Reference) (OtherActor :type Actor%20Object%20Reference) (OtherComp :type Primitive%20Component%20Object%20Reference) (OtherBodyIndex :type Integer) (bFromSweep :type Boolean) (SweepResult :type Hit%20Result%20Structure%20%28by%20ref%29))
  (if (Variables|Default|GetbIsActive)
    (bind _asbp_energy_sphere (Utilities|Casting|CastToBP_EnergySphere OtherActor))
    (if (== (Variables|/Game/LabPuzzleGame/PuzzleElements/EnergySphere/BP_EnergySphere.BP_EnergySphere_C|GetFieldsCount _asbp_energy_sphere) 0)
      (Default|Kill _asbp_energy_sphere))))

(event EventBeginPlay
  (if (Variables|Default|GetbIsActive)
    (Components|Activation|Activate (Variables|Default|GetNS_DissolvingField) false)
    (for _array_element (Collision|GetOverlappingActors (Variables|Default|GetBox) "/Game/LabPuzzleGame/PuzzleElements/EnergySphere/BP_EnergySphere.BP_EnergySphere_C" :!class /Script/Engine.PrimitiveComponent)
      (bind _asbp_energy_sphere (Utilities|Casting|CastToBP_EnergySphere _array_element))
      (Default|Kill _asbp_energy_sphere))))

(event EventActivate
  (params (Type :type EActivationType%20Enum :default "NewEnumerator0"))
  (bind _ns_dissolvingfield (Variables|Default|GetNS_DissolvingField))
  (Utilities|ActivationSwitch (Utilities|ReverseActivation Type (Variables|Default|GetbReverse)) (Variables|Default|GetbIsActive)
    (:TurnOn
      (Variables|Default|SetbIsActive true)
      (Components|Activation|Activate _ns_dissolvingfield false)
      (for _array_element (Collision|GetOverlappingActors (Variables|Default|GetBox) "/Game/LabPuzzleGame/PuzzleElements/EnergySphere/BP_EnergySphere.BP_EnergySphere_C" :!class /Script/Engine.PrimitiveComponent)
        (bind _asbp_energy_sphere (Utilities|Casting|CastToBP_EnergySphere _array_element))
        (Default|Kill _asbp_energy_sphere)))
    (:TurnOff
      (Variables|Default|SetbIsActive false)
      (Components|Activation|Deactivate _ns_dissolvingfield))))

(fn ConstructionScript)

(fn IsActive
  (return false))