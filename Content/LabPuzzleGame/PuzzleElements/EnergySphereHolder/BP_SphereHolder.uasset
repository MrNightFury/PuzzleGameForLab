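; BP_SphereHolder is a timed energy sphere holder puzzle element that powers its linked elements for a limited duration.
; When activated by Toggle or Turn on, or at BeginPlay if active, it starts the Niagara sphere and sends TurnOn to linked elements.
; A Timeline stretched to ActiveTime drives the sphere's orbScale, then clears IsActive and sends TurnOff when finished.
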(event EventBeginPlay
  (Components|Timeline|SetPlayRate (Variables|Default|GetTimeline) (/ 1.0 (Variables|Default|GetActiveTime)))
  (if (Variables|Default|GetbIsActive)
    (CallFunction|Start)))

(event EventTick
  (params (DeltaSeconds :type Float%20%28single-precision%29)))

(event EventActivate
  (params (Type :type EActivationType%20Enum :default "NewEnumerator0"))
  (switch Utilities|FlowControl|Switch|SwitchonEActivationType Type
    (:NewEnumerator0
      _)
    (:NewEnumerator1
      _))
  (CallFunction|Start)
  (Variables|Default|SetbIsActive true))

(fn ConstructionScript
  (|CallParentFunction))

(fn Start
  (Components|Activation|Activate (Variables|Default|GetNS_SphereHolder_Sphere) false)
  (Components|Timeline|PlayfromStart (Variables|Default|GetTimeline))
  (CallFunction|ActivateLinkedwithSpecificType "NewEnumerator1"))

(fn IsActive
  (return false))