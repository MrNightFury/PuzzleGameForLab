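; BP_EnergySphereReciever is a lab puzzle element that triggers linked elements when an energy sphere enters it.
; On box overlap, if receiver and sphere are both active, it calls ActivateLinked and the sphere's dispenser's Shoot.
; Any overlapping energy sphere is then destroyed.
; Activate toggles the receiver's IsActive flag, while the IsActive function always returns false.
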(event OnComponentBeginOverlap(Box)
  (params (OverlappedComponent :type Primitive%20Component%20Object%20Reference) (OtherActor :type Actor%20Object%20Reference) (OtherComp :type Primitive%20Component%20Object%20Reference) (OtherBodyIndex :type Integer) (bFromSweep :type Boolean) (SweepResult :type Hit%20Result%20Structure%20%28by%20ref%29))
  (bind _asbp_energy_sphere (Utilities|Casting|CastToBP_EnergySphere OtherActor))
  (if (and (Variables|Default|GetbIsActive) (Variables|/Game/LabPuzzleGame/PuzzleElements/EnergySphere/BP_EnergySphere.BP_EnergySphere_C|GetbIsActive _asbp_energy_sphere))
    (CallFunction|ActivateLinked)
    (Default|Shoot (Variables|/Game/LabPuzzleGame/PuzzleElements/EnergySphere/BP_EnergySphere.BP_EnergySphere_C|GetDispenser _asbp_energy_sphere) true))
  (Actor|DestroyActor _asbp_energy_sphere))

(event EventActivate
  (params (Type :type EActivationType%20Enum :default "NewEnumerator0"))
  (Variables|Default|SetbIsActive (not (Variables|Default|GetbIsActive))))

(fn ConstructionScript)

(fn IsActive
  (return false))