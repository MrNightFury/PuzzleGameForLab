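; Puzzle cube Blueprint that acts as a field, carrying a sphere along with its own motion.
; Do applies the cube's location and rotation change since the cached LastTransform to the given sphere as an unswept world transform, then refreshes the cache.
; Overlap begin and end extend parent behavior by incrementing and decrementing the sphere's FieldsCount.
; LastTransform is also reset on BeginPlay and each overlap begin.
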(event EventBeginPlay
  (|CallParentFunction)
  (Variables|Default|SetlastTransform (Transformation|GetActorTransform)))

(event EventTick
  (params (DeltaSeconds :type Float%20%28single-precision%29))
  (|CallParentFunction DeltaSeconds))

(fn ConstructionScript
  (|CallParentFunction))

(fn Do
  (params (Sphere :type BP%20Energy%20Sphere%20Object%20Reference) (Delta%20seconds :type Float%20%28double-precision%29))
  (bind _returnvalue (Transformation|GetActorTransform))
  (bind (_location _rotation) (Math|Transform|BreakTransform _returnvalue))
  (Class|Actor|AddActorWorldTransform Sphere (Math|Transform|MakeTransform (- _location (.Location (Math|Transform|BreakTransform (Variables|Default|GetlastTransform)))) (Math|Rotator|Delta(Rotator) _rotation (.Rotation (Math|Transform|BreakTransform (Variables|Default|GetlastTransform)))) (Class|KismetMathLibrary|VectorOne)) false false)
  (Variables|Default|SetlastTransform _returnvalue))

(fn BeginOverlap
  (params (Sphere :type BP%20Energy%20Sphere%20Object%20Reference))
  (|CallParentFunction Sphere)
  (Variables|Default|SetlastTransform (Transformation|GetActorTransform))
  (Math|Integer|IncrementInt (Variables|/Game/LabPuzzleGame/PuzzleElements/EnergySphere/BP_EnergySphere.BP_EnergySphere_C|GetFieldsCount Sphere)))

(fn EndOverlap
  (params (Sphere :type BP%20Energy%20Sphere%20Object%20Reference))
  (|CallParentFunction Sphere)
  (Math|Integer|DecrementInt (Variables|/Game/LabPuzzleGame/PuzzleElements/EnergySphere/BP_EnergySphere.BP_EnergySphere_C|GetFieldsCount Sphere)))