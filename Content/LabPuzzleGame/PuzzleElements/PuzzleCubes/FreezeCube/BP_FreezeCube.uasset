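; Freeze cube puzzle element that halts a sphere's physics motion when it overlaps the cube.
; Extends a parent cube's overlap handlers, zeroing the sphere collider's linear velocity on entry and setting it to the sphere's Speed on exit.
; BeginPlay passes the freeze effect's scaled world size into its Scale variable; a WindSpeed update exists but is unconnected.
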(event EventBeginPlay
  (bind _ns_cube_freeze (Variables|Default|GetNS_Cube_Freeze))
  ;[0.03529 0.03529 0.03529] Initial pass scale to NS
  (|CallParentFunction)
  (Niagara|SetNiagaraVariable(Vector3) _ns_cube_freeze "Scale" (* 48.0 (Transformation|GetWorldScale _ns_cube_freeze))))

(event EventTick
  (params (DeltaSeconds :type Float%20%28single-precision%29))
  (|CallParentFunction DeltaSeconds))

(fn ConstructionScript
  (|CallParentFunction))

(fn BeginOverlap
  (params (Sphere :type BP%20Energy%20Sphere%20Object%20Reference))
  (|CallParentFunction Sphere)
  (Physics|SetPhysicsLinearVelocity (Variables|/Game/LabPuzzleGame/PuzzleElements/EnergySphere/BP_EnergySphere.BP_EnergySphere_C|GetSphereCollider Sphere) "0, 0, 0" false "None"))

(fn EndOverlap
  (params (Sphere :type BP%20Energy%20Sphere%20Object%20Reference))
  (|CallParentFunction Sphere)
  (Physics|SetPhysicsLinearVelocity (Variables|/Game/LabPuzzleGame/PuzzleElements/EnergySphere/BP_EnergySphere.BP_EnergySphere_C|GetSphereCollider Sphere) (Variables|/Game/LabPuzzleGame/PuzzleElements/EnergySphere/BP_EnergySphere.BP_EnergySphere_C|GetSpeed Sphere) false "None"))