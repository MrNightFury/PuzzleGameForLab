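; BP_SpeedCube is a puzzle cube that changes a sphere's velocity, with a Niagara wind-style effect showing the push.
; Its Do function adds the SpeedChange vector, scaled by delta time, to the sphere's speed as a steady acceleration.
; BeginPlay passes the effect's world scale and the SpeedChange magnitude into NSCubeSpeed as Scale and WindSpeed, and prints that magnitude.
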(event EventBeginPlay
  (bind _ns_cube_speed (Variables|Default|GetNS_Cube_Speed))
  (bind _speedchange (Variables|Default|GetSpeedChange))
  (bind _returnvalue (Math|Vector|VectorLength _speedchange))
  ;[0.03529 0.03529 0.03529] Initial pass scale to NS
  (|CallParentFunction)
  (Niagara|SetNiagaraVariable(Vector3) _ns_cube_speed "Scale" (* 48.0 (Transformation|GetWorldScale _ns_cube_speed)))
  (Niagara|SetNiagaraVariable(Float) _ns_cube_speed "WindSpeed" _returnvalue)
  (Development|PrintString (Utilities|String|ToString(Float) _returnvalue)))

(fn ConstructionScript
  (|CallParentFunction))

(fn Do
  (params (Sphere :type BP%20Energy%20Sphere%20Object%20Reference) (Delta%20seconds :type Float%20%28double-precision%29))
  (Default|AddSpeed Sphere (* Delta%20seconds (Variables|Default|GetSpeedChange))))