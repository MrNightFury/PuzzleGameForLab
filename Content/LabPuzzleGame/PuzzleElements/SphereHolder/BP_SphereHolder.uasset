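; BP_SphereHolder is a lab puzzle element that holds an energy sphere and powers linked elements once active.
; It activates on begin play if flagged, or later through its Activate event when not already active.
; Activation starts a timer calling ActivateLinked by name, optionally looping, and turns on the energy sphere Niagara effect.
; The construction script only runs the parent's.
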(event EventBeginPlay
  (if (Variables|Default|GetbAsActiveOnStart)
    (Utilities|Time|SetTimerbyFunctionName 0 "ActivateLinked" (Variables|Default|GetPeriod) (Variables|Default|GetbIsLooping))
    (Variables|Default|SetbIsActive true)
    (Components|Activation|Activate (Variables|Default|GetNS_EnergySphere) false)))

(event EventActivate
  (if (not (Variables|Default|GetbIsActive))
    (Utilities|Time|SetTimerbyFunctionName 0 "ActivateLinked" (Variables|Default|GetPeriod) (Variables|Default|GetbIsLooping))
    (Variables|Default|SetbIsActive true)
    (Components|Activation|Activate (Variables|Default|GetNS_EnergySphere) false)))

(fn ConstructionScript
  (|CallParentFunction))